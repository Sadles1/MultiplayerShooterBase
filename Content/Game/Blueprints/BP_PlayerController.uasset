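; BP_PlayerController is the player controller that links input, HUD widgets and game mode requests.
; Interact input calls ServerInteract, while menu inputs toggle the spawn-weapon and map-select widgets through HUD messages.
; Client events add or remove the weapon info widget on the HUD.
; Server events cast to BP_GameMode to respawn the player or switch maps.
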(event Custom|Client_AddWeaponInfoWidget
  (params (Weapon :type Base%20Weapon%20Object%20Reference))
  (Class|BPIHUD|AddWeaponInfoWidget(Message) (HUD|GetHUD) Weapon))

(event Custom|Client_RemoveWeaponInfoWidget
  (Class|BPIHUD|RemoveWeaponInfoWidget(Message) (HUD|GetHUD)))

(event Custom|Server_RespawnPlayer
  (bind _asbp_game_mode (Utilities|Casting|CastToBP_GameMode (Game|GetGameMode)))
  (Class|MSGameMode|RespawnPlayer _asbp_game_mode self))

(event Custom|Server_SwitchMap
  (params (NewMap :type Name))
  (bind _asbp_game_mode (Utilities|Casting|CastToBP_GameMode (Game|GetGameMode)))
  (Default|SwitchMap _asbp_game_mode NewMap))

(event Input|ActionEvents|InputActionInteract
  (params (Key :type Key%20Structure :default "None"))
  (:Pressed
    (Class|BasePlayerController|ServerInteract)))

(event Input|ActionEvents|InputActionSpawnWeaponMenu
  (params (Key :type Key%20Structure :default "None"))
  (:Pressed
    (Class|BPIHUD|ToggleSpawnWeaponWidget(Message) (HUD|GetHUD))))

(event Input|ActionEvents|InputActionMapSelectMenu
  (params (Key :type Key%20Structure :default "None"))
  (:Pressed
    (Class|BPIHUD|ToggleMapSelectWidget(Message) (HUD|GetHUD))))

(fn ConstructionScript)