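; BP_PlayerCharacter is the player character Blueprint, handling movement, look and item-use input.
; Axis inputs drive movement along the actor's forward and right vectors and add controller yaw and pitch.
; Pressing and releasing Use call server start and stop functions for the current item, which are not defined in these graphs.
; The death event only prints a debug string, and the construction script is empty.
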(event EventOnDeath
  (Development|PrintString "Death"))

(event Input|ActionEvents|InputActionUse
  (params (Key :type Key%20Structure :default "None"))
  (:Pressed
    (Class|BasePlayerCharacter|ServerStartUseCurrentItem))
  (:Released
    (Class|BasePlayerCharacter|ServerStopUseCurrentItem)))

(event Input|AxisEvents|InputAxisMoveForward
  (params (AxisValue :type Float%20%28single-precision%29))
  ;[1 1 1] Movement
  (Pawn|Input|AddMovementInput (Transformation|GetActorForwardVector) AxisValue false))

(event Input|AxisEvents|InputAxisMoveRight
  (params (AxisValue :type Float%20%28single-precision%29))
  ;[1 1 1] Movement
  (Pawn|Input|AddMovementInput (Transformation|GetActorRightVector) AxisValue false))

(event Input|AxisEvents|InputAxisLookUp
  (params (AxisValue :type Float%20%28single-precision%29))
  ;[1 1 1] Movement
  (Pawn|Input|AddControllerPitchInput AxisValue))

(event Input|AxisEvents|InputAxisTurn
  (params (AxisValue :type Float%20%28single-precision%29))
  ;[1 1 1] Movement
  (Pawn|Input|AddControllerYawInput AxisValue))

(fn ConstructionScript)